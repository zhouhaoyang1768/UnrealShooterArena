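; BP_HealthComponent is an actor component that tracks health through current and maximum HP.
; Damage lowers current HP down to zero unless a temporary immunity timer is running, and Heal raises it up to the maximum.
; SetImmuneTIme starts the immunity window, which Tick counts down, and GetHealthPercentage returns current HP as a fraction of the maximum.
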(event Custom|Damage
  (params (damage :type Float%20%28double-precision%29))
  (if (<= (Variables|Default|GetImmuneTime) 0.0)
    (Variables|Default|SetCurrentHP (Math|Float|Max(Float) (- (Variables|Default|GetCurrentHP) damage) 0.0))))

(event Custom|Heal
  (params (amount :type Float%20%28double-precision%29))
  (Variables|Default|SetCurrentHP (Math|Float|Min(Float) (+ amount (Variables|Default|GetCurrentHP)) (Variables|Default|GetMaxHP))))

(event Custom|Set%20Immune%20TIme
  (params (seconds :type Float%20%28double-precision%29))
  (Variables|Default|SetImmuneTime seconds))

(event EventBeginPlay)

(event EventTick
  (params (DeltaSeconds :type Float%20%28single-precision%29))
  (Variables|Default|SetImmuneTime (Math|Float|Max(Float) (- (Variables|Default|GetImmuneTime) DeltaSeconds) 0.0)))

(fn GetHealthPercentage
  (return (/ (Variables|Default|GetCurrentHP) (Variables|Default|GetMaxHP))))